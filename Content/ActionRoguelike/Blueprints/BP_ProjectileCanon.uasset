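; BP_ProjectileCanon is a turret-style actor that periodically fires BP_MagicProjectile.
; A looping timer started on BeginPlay spawns a projectile at the actor's location every two seconds.
; Tick turns the Arrow component to face the first player's pawn, but projectiles spawn with the actor's own rotation, so that aim does not feed into the shot.
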(event `self.ReceiveTick`
  (params (DeltaSeconds :type "Float (single-precision)"))
  (`SceneComponent.K2_SetWorldRotation` (`self.Arrow`) (`KismetMathLibrary.FindLookAtRotation` (`self.K2_GetActorLocation`) (`self.K2_GetActorLocation` (`GameplayStatics.GetPlayerPawn` 0))) false false))

(event `self.ReceiveBeginPlay`
  (`KismetSystemLibrary.K2_SetTimerDelegate` (delegate `OnTimerElapsed`) 2.0 true))

(event `OnTimerElapsed`
  (`|SpawnActorFromClass` "/Game/ActionRoguelike/Blueprints/BP_MagicProjectile.BP_MagicProjectile_C" (`KismetMathLibrary.MakeTransform` (`self.K2_GetActorLocation`) (`self.K2_GetActorRotation`)) "Undefined" "OverrideRootScale" null null))

(fn `UserConstructionScript`)